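; Player pawn Blueprint that assembles the player's body from separate meshes and forwards controller trigger input.
; On begin play, Body, Arms and Head follow the IK component's pose, while both hands, a watch and a credit card attach to Arms sockets.
; It hands the camera and IK component to the BP_Player_Anim animation instance for IK.
; Each tick it passes right and left trigger readings to SetTriggerValues.
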(event `self.ReceiveBeginPlay`
  ;[1 1 1] at begin play sync skeletons
  (`SkinnedMeshComponent.SetLeaderPoseComponent` (`self.Body`) (`self.IK`) false false)
  (`SkinnedMeshComponent.SetLeaderPoseComponent` (`self.Arms`) (`self.IK`) false false)
  (`SkinnedMeshComponent.SetLeaderPoseComponent` (`self.Head`) (`self.IK`) false false)
  ;[1 1 1] at begin play attach hands, watch and credit card to sockets
  (`SceneComponent.K2_AttachToComponent` (`self.RightHand`) (`self.Arms`) "Socket_RightHand" "SnapToTarget" "KeepRelative" "KeepRelative" true)
  (`SceneComponent.K2_AttachToComponent` (`self.LeftHand`) (`self.Arms`) "Socket_LeftHand" "SnapToTarget" "KeepRelative" "KeepRelative" true)
  (`SceneComponent.K2_AttachToComponent` (`self.Watch`) (`self.Arms`) "Socket_LeftLowerArm" "SnapToTarget" "KeepRelative" "KeepRelative" true)
  (`SceneComponent.K2_AttachToComponent` (`self.CreditCard`) (`self.Arms`) "Socket_RightHand" "KeepRelative" "KeepRelative" "KeepRelative" true)
  ;[1 1 1] at begin play set references in animation blueprint for IK
  (bind _asbp_player_anim (cast `/Game/Character/Player/Animation/BP_Player_Anim` (`SkeletalMeshComponent.GetAnimInstance` (`self.IK`))))
  (set `/Game/Character/Player/Animation/BP_Player_Anim.Camera` (`self.Camera`) _asbp_player_anim)
  (set `/Game/Character/Player/Animation/BP_Player_Anim.IK` (`self.IK`) _asbp_player_anim))

(event `self.ReceiveTick`
  (params (DeltaSeconds :type "Float (single-precision)"))
  ;[1 1 1] set trigger values from controller
  (`self.SetTriggerValues` (`KismetMathLibrary.MakeVector2D` (`self.GetInputAxisValue`) (`self.GetInputAxisValue`))))

(fn `UserConstructionScript`)